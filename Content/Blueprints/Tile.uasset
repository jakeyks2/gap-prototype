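; Tile is a clickable board tile actor that tracks its neighboring tiles.
; On click release it casts the player pawn to Player and passes itself to OnClickTile, leaving the response to the player.
; UpdateAdjacentTiles rebuilds AdjacentTiles from a supplied tile list, using a fixed distance threshold rather than grid indices and excluding itself.
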(event `self.ReceiveActorOnReleased`
  (params (ButtonReleased :type "Key Structure"))
  (bind _asplayer (cast `/Game/Blueprints/Player` (`GameplayStatics.GetPlayerPawn` 0)))
  (`/Game/Blueprints/Player.OnClickTile` _asplayer self))

(fn `UpdateAdjacentTiles`
  (params (AllTiles :type "Array of /Game/Blueprints/Tile Object Reference"))
  (bind _adjacenttiles (`self.AdjacentTiles`))
  (`KismetArrayLibrary.Array_Clear` _adjacenttiles)
  (for _array_element AllTiles
    (if (< (`self.GetDistanceTo` _array_element) 185.0)
      (`KismetArrayLibrary.Array_Add` (`self.AdjacentTiles`) _array_element)))
  (`KismetArrayLibrary.Array_RemoveItem` _adjacenttiles self))

(fn `UserConstructionScript`)