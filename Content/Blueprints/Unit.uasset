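; Unit actor for a tile-based game that occupies one tile and can be clicked by the player.
; A left-click release on the unit notifies the Player pawn through OnClickUnit.
; Move refuses an occupied target tile, otherwise it swaps the CurrentUnit and CurrentTile references, snaps the actor to the tile's location and returns success.
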(event `self.ReceiveActorOnReleased`
  (params (ButtonReleased :type "Key Structure"))
  (if (== ButtonReleased "LeftMouseButton")
    (bind _asplayer (cast `/Game/Blueprints/Player` (`GameplayStatics.GetPlayerPawn` 0)))
    (`/Game/Blueprints/Player.OnClickUnit` _asplayer self)))

(fn `Move`
  (params (TargetTile :type "/Game/Blueprints/Tile Object Reference"))
  (returns (Success :type Boolean))
  (`/Engine/EditorBlueprintResources/StandardMacros.IsValid` (`/Game/Blueprints/Tile.CurrentUnit` TargetTile)
    (:`Is Valid`
      (return false))
    (:`Is Not Valid`
      (set `/Game/Blueprints/Tile.CurrentUnit` null (`self.CurrentTile`))
      (set `/Game/Blueprints/Tile.CurrentUnit` self TargetTile)
      (bind _output_get (set `self.CurrentTile` TargetTile))
      (`self.K2_SetActorLocation` (`self.K2_GetActorLocation` _output_get))
      (return true))))

(fn `UserConstructionScript`)