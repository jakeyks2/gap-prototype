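; Player pawn for a tile-based battle, providing a movable spring-arm camera and click-to-move unit control.
; Axis inputs move and zoom; holding TurnCamera hides the cursor and enables yaw on the actor and pitch on the arm.
; OnClickUnit gathers tiles within two adjacency steps, highlighting the unit and unoccupied tiles.
; OnClickTile moves the unit to any gathered tile, without rechecking occupancy, and deselects either way.
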(event `self.ReceiveBeginPlay`
  (bind _asbattle_controller (cast `/Game/Blueprints/BattleController` (`self.GetController`)))
  (bind _output_get (set `self.BattleController` _asbattle_controller))
  (`WidgetBlueprintLibrary.SetInputMode_GameAndUIEx` _output_get null))

(event `InputAxis|MoveForward`
  (params (AxisValue :type "Float (single-precision)"))
  (`self.AddMovementInput` (`self.GetActorForwardVector`) AxisValue))

(event `InputAxis|MoveRight`
  (params (AxisValue :type "Float (single-precision)"))
  (`self.AddMovementInput` (`self.GetActorRightVector`) AxisValue))

(event `InputAxis|Zoom`
  (params (AxisValue :type "Float (single-precision)"))
  (bind _output_get (set `SpringArmComponent.TargetArmLength` (- (stale _output_get) (* AxisValue 50.0)) (`self.SpringArm`))))

(event `InputAxis|Rotate`
  (params (AxisValue :type "Float (single-precision)"))
  (bind (_returnvalue_roll _returnvalue_pitch _returnvalue_yaw) (`KismetMathLibrary.BreakRotator` (`self.GetControlRotation`)))
  (if (`self.bIsTurningCamera`)
    (`self.AddControllerYawInput` (* AxisValue 0.5))
    (`self.K2_SetActorRotation` (`KismetMathLibrary.MakeRotator` 0.0 0.0 _returnvalue_yaw))))

(event `InputAxis|Pitch`
  (params (AxisValue :type "Float (single-precision)"))
  (bind (_returnvalue_roll _returnvalue_pitch) (`KismetMathLibrary.BreakRotator` (`self.GetControlRotation`)))
  (if (`self.bIsTurningCamera`)
    (`self.AddControllerPitchInput` (* AxisValue -0.5))
    (`SceneComponent.K2_SetRelativeRotation` (`self.SpringArm`) (`KismetMathLibrary.MakeRotator` 0.0 _returnvalue_pitch) false false)))

(event `InputAction|TurnCamera`
  (params (Key :type "Key Structure"))
  (bind _battlecontroller (`self.BattleController`))
  (:`Pressed`
    (set `self.bIsTurningCamera` true)
    (set `PlayerController.bShowMouseCursor` false _battlecontroller))
  (:`Released`
    (set `self.bIsTurningCamera` false)
    (set `PlayerController.bShowMouseCursor` true _battlecontroller)))

(fn `Deselect`
  (set `self.bIsMovingUnit` false)
  (`SceneComponent.SetVisibility` (`/Game/Blueprints/Unit.Highlight` (`self.UnitBeingMoved`)) false false)
  (for _array_element (`self.UnitDestinations`)
    (`SceneComponent.SetVisibility` (`/Game/Blueprints/Tile.Highlight` _array_element) false false)))

(fn `OnClickTile`
  (params (Tile :type "/Game/Blueprints/Tile Object Reference"))
  (if (`self.bIsMovingUnit`)
    (if (`KismetArrayLibrary.Array_Contains` (`self.UnitDestinations`) Tile)
      (`/Game/Blueprints/Unit.Move` (`self.UnitBeingMoved`) Tile)
      (`self.Deselect`)
      (else
        (`self.Deselect`)))))

(fn `OnClickUnit`
  (params (Unit :type "/Game/Blueprints/Unit Object Reference"))
  (`/Engine/EditorBlueprintResources/StandardMacros.IsValid` (`self.UnitBeingMoved`)
    (:`Is Valid`
      (`self.Deselect`))
    (:`Is Not Valid`
      _))
  (set `self.bIsMovingUnit` true)
  (bind _output_get (set `self.UnitBeingMoved` Unit))
  (`SceneComponent.SetVisibility` (`/Game/Blueprints/Unit.Highlight` _output_get) true false)
  (bind _currenttile (`/Game/Blueprints/Unit.CurrentTile` _output_get))
  (bind _adjacenttiles (`/Game/Blueprints/Tile.AdjacentTiles` _currenttile))
  (bind _output_get_2 (set `self.UnitDestinations` _adjacenttiles))
  (for _array_element _adjacenttiles
    (for _array_element_2 (`/Game/Blueprints/Tile.AdjacentTiles` _array_element)
      (`KismetArrayLibrary.Array_AddUnique` _output_get_2 _array_element_2)))
  (`KismetArrayLibrary.Array_RemoveItem` _output_get_2 _currenttile)
  (for _array_element_3 _output_get_2
    (`/Engine/EditorBlueprintResources/StandardMacros.IsValid` (`/Game/Blueprints/Tile.CurrentUnit` _array_element_3)
      (:`Is Not Valid`
        (`SceneComponent.SetVisibility` (`/Game/Blueprints/Tile.Highlight` _array_element_3) true false)))))

(fn `UserConstructionScript`)